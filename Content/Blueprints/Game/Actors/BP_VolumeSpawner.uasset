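; BP_VolumeSpawner is an actor that keeps spawning BP_Card actors inside a box volume.
; On BeginPlay it starts a looping timer that fires SpawnCard, placing each card at a random point within the scaled box bounds with zero rotation.
; The construction script applies the BoxExtent variable to the Box component, which sets the size of the spawn area.
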(event Custom|SpawnCard
  (Game|SpawnActorfromClass "/Game/Blueprints/Game/Actors/BP_Card.BP_Card_C" (Math|Transform|MakeTransform (Math|Random|RandomPointinBoundingBox (Transformation|GetWorldLocation (Variables|Default|GetBox)) (Components|Box|GetScaledBoxExtent (Variables|Default|GetBox)))) "Undefined" "MultiplyWithRoot" 0 0))

(event EventBeginPlay
  (Utilities|Time|SetTimerbyEvent (delegate Custom|SpawnCard) 0.8 true))

(fn ConstructionScript
  (Components|Box|SetBoxExtent (Variables|Default|GetBox) (Variables|UserDefined|GetBoxExtent) true))