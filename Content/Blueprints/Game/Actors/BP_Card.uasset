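; BP_Card is a card actor that carries a color and an answer text and reports both to the L1_GameMode.
; On BeginPlay it reads the answer string from the WBP_AnswerText widget in its CardTextWidget component and caches it.
; NewFunction finds the game mode with GetActorOfClass and passes Color and Answer through ColorTunnel and TextTunnel.
; The click handler is empty and its binding is unconnected.
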(event Custom|OnClicked_Event
  (params (TouchedActor :type Actor%20Object%20Reference) (ButtonPressed :type Key%20Structure :default "None")))

(event EventBeginPlay
  (bind _aswbp_answer_text (Utilities|Casting|CastToWBP_AnswerText (UserInterface|GetUserWidgetObject (Variables|Default|GetCardTextWidget))))
  (Variables|Default|SetAnswer (Variables|/Script/UMG.TextBlock|GetText (Variables|/Game/UMG/Game/WBP_AnswerText.WBP_AnswerText_C|GetAnswerText _aswbp_answer_text))))

(event Collision|EventActorBeginOverlap
  (params (OtherActor :type Actor%20Object%20Reference)))

(event EventTick
  (params (DeltaSeconds :type Float%20%28single-precision%29)))

(event EventNewFunction
  (bind _returnvalue (Actor|GetActorOfClass "/Game/Blueprints/Game/Level1/L1_GameMode.L1_GameMode_C"))
  (Default|ColorTunnel _returnvalue (Variables|Default|GetColor))
  (Default|TextTunnel _returnvalue (Variables|Default|GetAnswer)))

(fn ConstructionScript)