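; Player controller for a click-to-shoot game that destroys actors under the mouse cursor.
; On BeginPlay it shows the cursor and adds the CG_IMC Enhanced Input mapping context.
; IA_Shoot deprojects the cursor and line-traces on Visibility, with the end point built from the direction alone, not offset from the start.
; A hit actor receives NewFunctionMessage, then ChangeBackgroundColor is called and the actor is destroyed.
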(event Input|EnhancedActionEvents|EnhancedInputActionIA_Shoot
  (params (ActionValue :type Boolean) (ElapsedSeconds :type Float%20%28double-precision%29) (TriggeredSeconds :type Float%20%28double-precision%29) (InputAction :type Input%20Action%20Object%20Reference :default "/Game/Input/Actions/IA_Shoot.IA_Shoot"))
  (bind (_worldlocation _worlddirection) (Game|Player|ConvertMouseLocationToWorldSpace))
  (:Started
    (bind _outhit (Collision|LineTraceByChannel _worldlocation (+ _worlddirection (* _worlddirection 1e+04)) "TraceTypeQuery1" false 0 "None"))
    (Utilities|IsValid (.HitActor (Collision|BreakHitResult _outhit))
      (:Is%20Valid
        (Class|L1Interface|NewFunction(Message) (.HitActor (Collision|BreakHitResult _outhit)))
        (Default|CallChangeBackgroundColor)
        (Actor|DestroyActor (.HitActor (Collision|BreakHitResult _outhit)))))))

(event EventBeginPlay
  (bind _returnvalue (PlayerController|LocalPlayerSubsystems|GetEnhancedInputLocalPlayerSubsystem))
  (Variables|Default|SetbShowMouseCursor true)
  (Utilities|IsValid _returnvalue
    (:Is%20Valid
      (Input|AddMappingContext _returnvalue "/Game/Input/CG_IMC.CG_IMC" 0 "(bIgnoreAllPressedKeysUntilRelease=True,bForceImmediately=False,bNotifyUserSettings=False)"))))

(fn ConstructionScript)